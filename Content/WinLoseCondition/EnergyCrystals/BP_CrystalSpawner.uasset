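; Spawner actor that creates BP_EnergyCrystal pickups at random reachable navmesh points within a small radius of itself.
; BeginPlay counts down from a fixed crystal total, setting the same looping half-second timer on each pass.
; Repeated calls only reset that one timer, so each tick spawns one crystal indefinitely and the count does not cap spawning.
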(event `self.ReceiveBeginPlay`
  (set `self.EnergyCrystalCounter` 20)
  (set `self.CrystalstoSpawn` (`self.EnergyCrystalCounter`))
  (if (> (`self.CrystalstoSpawn`) 0) :!label _label
    (`KismetSystemLibrary.K2_SetTimerDelegate` (delegate `SpawnCrystals`) 0.5 true)
    (`/Engine/EditorBlueprintResources/StandardMacros.DecrementInt` (`self.CrystalstoSpawn`)
      (:`  `
        (goto _label)))))

(event `SpawnCrystals`
  (`|SpawnActorFromClass` "/Game/WinLoseCondition/EnergyCrystals/BP_EnergyCrystal.BP_EnergyCrystal_C" (`KismetMathLibrary.Conv_VectorToTransform` (`NavigationSystemV1.K2_GetRandomReachablePointInRadius` (`self.K2_GetActorLocation`) 5.0 null null)) "Undefined" "MultiplyWithRoot" null null))

(fn `UserConstructionScript`)