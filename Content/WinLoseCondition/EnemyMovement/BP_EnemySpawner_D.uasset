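; BP_EnemySpawner_D is an enemy spawner actor that periodically creates BP_EnemyAI enemies.
; On BeginPlay it starts a looping ten-second timer that fires SpawnEnemy.
; Each firing loops to spawn a batch of enemies, all at the spawner's own location with no offset and default collision handling.
; Nothing caps or stops the spawning, and an offset-transform calculation is left unused.
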(event `self.ReceiveBeginPlay`
  (`KismetSystemLibrary.K2_SetTimerDelegate` (delegate `Spawn Enemy`) 10.0 true))

(event `Spawn Enemy`
  (for _ (range 11)
    (`|SpawnActorFromClass` "/Game/Enemy/BP_EnemyAI.BP_EnemyAI_C" (`KismetMathLibrary.Conv_VectorToTransform` (`self.K2_GetActorLocation`)) "Undefined" "MultiplyWithRoot" null null)))

(fn `UserConstructionScript`)