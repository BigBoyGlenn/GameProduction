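; BP_NewEnemyBase is an enemy base Blueprint that walks through an ordered array of waypoint actors.
; On BeginPlay it spawns its default controller, waits briefly, then issues AI MoveTo toward the waypoint at the current index.
; Each success increments the index and calls the Move event to repeat the request.
; The index has no wrap or bounds check, and failed moves are not handled.
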(event `self.ReceiveBeginPlay`
  (`self.SpawnDefaultController`)
  (`KismetSystemLibrary.Delay` 0.2)
  (`|AIMoveTo` self (`self.K2_GetActorLocation` (`|GetArrayItem` (`self.Waypoints`) (`self.Pos`))) null :!label _label
    (:`OnSuccess`
      (`/Engine/EditorBlueprintResources/StandardMacros.IncrementInt` (`self.Pos`)
        (:`  `
          (`self.Move`))))))

(event `Move`
  (goto _label))

(fn `UserConstructionScript`)