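; BP_EnemyAI_W is a crystal-thief enemy that heads for energy crystals and retreats with them.
; Each Tick it moves toward the first BP_EnergyCrystal found, or BP_CrystalCollision when none exist.
; While HoldingCrystal, set true outside this graph, it returns toward BP_EnemySpawner_W and destroys itself on arrival.
; A BP_Projectile overlap destroys the enemy, respawning a held crystal; the projectile's destroy node is unconnected.
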(event `self.ReceiveBeginPlay`
  (set `self.HoldingCrystal?` false)
  (bind _returnvalue (`GameplayStatics.GetActorOfClass` "/Game/Enemy/BP_EnemySpawner_W.BP_EnemySpawner_W_C")))

(event `self.ReceiveTick`
  (params (DeltaSeconds :type "Float (single-precision)"))
  (if (`self.HoldingCrystal?`)
    (`|AIMoveTo` self (`self.K2_GetActorLocation` (stale `self.ReceiveBeginPlay` _returnvalue)) null 1000.0
      (:`OnSuccess`
        (`self.K2_DestroyActor`)))
    (else
      (bind _outactors (`GameplayStatics.GetAllActorsOfClass` "/Game/WinLoseCondition/EnergyCrystals/BP_EnergyCrystal.BP_EnergyCrystal_C"))
      (bind _returnvalue (`GameplayStatics.GetActorOfClass` "/Game/WinLoseCondition/EnergyCrystals/BP_EnergyCrystal.BP_EnergyCrystal_C"))
      (bind _returnvalue_2 (`GameplayStatics.GetActorOfClass` "/Game/WinLoseCondition/EnergyCrystals/BP_CrystalCollision.BP_CrystalCollision_C"))
      (if (> (`KismetArrayLibrary.Array_Length` _outactors) 0)
        (`|AIMoveTo` self (`self.K2_GetActorLocation` _returnvalue) null 70.0)
        (else
          (`|AIMoveTo` self (`self.K2_GetActorLocation` _returnvalue_2) null 70.0))))))

(event `self.ReceiveActorBeginOverlap`
  (params (OtherActor :type "Actor Object Reference"))
  (bind _asbp_projectile (cast `/Game/Blueprints/BP_Projectile` OtherActor))
  (if (`self.HoldingCrystal?`)
    (`|SpawnActorFromClass` "/Game/WinLoseCondition/EnergyCrystals/BP_EnergyCrystal.BP_EnergyCrystal_C" (`KismetMathLibrary.Conv_VectorToTransform` (`KismetMathLibrary.TransformLocation` (`self.GetTransform`) (0.0 0.0 -10.0))) "Undefined" "MultiplyWithRoot" null null))
  (`self.K2_DestroyActor`))

(fn `UserConstructionScript`)