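; Enemy turret Blueprint that detects the player character and fires projectiles at a limited rate.
; PawnSensing sightings of a PlayerCharacter set the actor's rotation from a look-at computed from the player's location toward the turret.
; Each sighting spawns BP_Projectile at the ProjectileDirection component's transform when CanAttack allows, with a short Delay resetting that flag.
; Debug strings print on sighting and firing.
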(event `self.PawnSensing.OnSeePawn`
  (params (Pawn :type "Pawn Object Reference"))
  (`KismetSystemLibrary.PrintString` "Hello")
  (bind _asplayer_character (cast `PlayerCharacter` Pawn))
  (`self.K2_SetActorRotation` (`KismetMathLibrary.FindRelativeLookAtRotation` (`KismetMathLibrary.Conv_VectorToTransform` (`self.K2_GetActorLocation` _asplayer_character)) (`self.K2_GetActorLocation`)))
  (if (`self.CanAttack`)
    (`KismetSystemLibrary.PrintString` "Goodbye")
    (`|SpawnActorFromClass` "/Game/Blueprints/BP_Projectile.BP_Projectile_C" (`SceneComponent.K2_GetComponentToWorld` (`self.ProjectileDirection`)) "Undefined" "MultiplyWithRoot" null null)
    (set `self.CanAttack` false)
    (`KismetSystemLibrary.Delay` 0.1)
    (set `self.CanAttack` true)))

(fn `UserConstructionScript`)