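; Player-owned turret actor that automatically shoots at enemy pawns it sees.
; PawnSensing's See Pawn event passes dragon, wizard, turtle or base enemy casts into one shared path that snaps rotation toward the target and spawns BP_Projectile at ProjectileDirection.
; A CanAttack flag and delay form the fire cooldown.
; An older CanSee-based targeting branch and debug prints are left disconnected.
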(event `self.ReceiveTick`
  (params (DeltaSeconds :type "Float (single-precision)"))
  ;[1 1 1] Overcomplicated turret
)

(event `CustomEvent`
  (params (Pawn :type "Pawn Object Reference"))
  ;[1 1 1] Overcomplicated turret
  (cast `/Game/Enemy/RawVersion/BP_EnemyBase` Pawn
    (:`then`
      (set `self.CanSee` true))
    (:`CastFailed`
      (set `self.CanSee` false))))

(event `self.PawnSensing.OnSeePawn`
  (params (Pawn :type "Pawn Object Reference"))
  (if (`self.CanAttack`)
    (cast `/Game/Enemy/RawVersion/BP_EnemyDragon` Pawn
      (:`then`
        _)
      (:`CastFailed`
        (cast `/Game/Enemy/RawVersion/BP_EnemyWizard` Pawn
          (:`then`
            _)
          (:`CastFailed`
            (cast `/Game/Enemy/RawVersion/BP_EnemyTurtle` Pawn
              (:`then`
                _)
              (:`CastFailed`
                (cast `/Game/Enemy/RawVersion/BP_EnemyBase` Pawn)))))))
    (`self.K2_SetActorRotation` (`KismetMathLibrary.FindRelativeLookAtRotation` (`KismetMathLibrary.Conv_VectorToTransform` (`self.K2_GetActorLocation`)) (`self.K2_GetActorLocation` Pawn)))
    (`|SpawnActorFromClass` "/Game/Blueprints/BP_Projectile.BP_Projectile_C" (`SceneComponent.K2_GetComponentToWorld` (`self.ProjectileDirection`)) "Undefined" "MultiplyWithRoot" null null)
    (set `self.CanAttack` false)
    (`KismetSystemLibrary.Delay` 1.0)
    (set `self.CanAttack` true)))

(fn `UserConstructionScript`)