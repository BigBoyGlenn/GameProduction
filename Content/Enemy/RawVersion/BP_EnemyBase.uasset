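; Enemy base actor that walks to the crystal, steals it and carries it back to its spawn point.
; On BeginPlay it spawns its controller and chains two AIMoveTo calls, calling TakeCrystal and showing a stolen-crystal component at the crystal, then destroying itself on return.
; Overlapping projectiles are destroyed and update HP from a decremented BaseDamage value, printing it and destroying the enemy at zero or below.
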(event `self.ReceiveBeginPlay`
  (set `self.Start` (`self.K2_GetActorLocation`))
  (`self.SpawnDefaultController`)
  (bind _returnvalue (`GameplayStatics.GetActorOfClass` "/Game/WinLoseCondition/EnergyCrystals/BP_CrystalCollision.BP_CrystalCollision_C"))
  (`|AIMoveTo` self (`self.K2_GetActorLocation` _returnvalue) null 10.0
    (:`OnSuccess`
      (bind _returnvalue_2 (`GameplayStatics.GetActorOfClass` "/Game/WinLoseCondition/EnergyCrystals/BP_CrystalCollision.BP_CrystalCollision_C"))
      (`/Game/WinLoseCondition/EnergyCrystals/BP_CrystalCollision.TakeCrystal` _returnvalue_2)
      (`SceneComponent.SetVisibility` (`self.StolenCrystal`) true false)
      (`|AIMoveTo` self (`self.Start`) null 10.0
        (:`OnSuccess`
          (`self.K2_DestroyActor`))))))

(event `self.ReceiveActorBeginOverlap`
  (params (OtherActor :type "Actor Object Reference"))
  (bind _asbp_projectile (cast `/Game/Blueprints/BP_Projectile` OtherActor))
  (`self.K2_DestroyActor` _asbp_projectile)
  (bind _result (`/Engine/EditorBlueprintResources/StandardMacros.DecrementFloat` (`self.BaseDamage`))
    (:`  `
      (bind _output_get (set `self.HP` _result))
      (`KismetSystemLibrary.PrintString` (`KismetStringLibrary.Conv_DoubleToString` _output_get))
      (if (<= _output_get 0.0)
        (`self.K2_DestroyActor`)))))

(fn `UserConstructionScript`)