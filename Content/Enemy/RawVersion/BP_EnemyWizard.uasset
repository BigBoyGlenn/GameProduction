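; Wizard enemy that summons minions while trying to steal the crystal and carry it back to its spawn point.
; It spawns BP_EnemyBase batches on a delayed loop gated by Slime, which is set from BaseDamage rather than its own count.
; AI movement retries until it reaches BP_CrystalCollision, takes the crystal, then returns and despawns.
; Projectile hits flash its material and subtract HP; death while carrying drops a BP_EnergyCrystal.
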(event `Summon Slime!`
  ;[1 1 1] Wizard spawning in enemies
  (if (not (>= (`self.Slime`) 10)) :!label _label
    (`KismetSystemLibrary.Delay` 10.0)
    (for _ (range 4)
      (`|SpawnActorFromClass` "/Game/Enemy/RawVersion/BP_EnemyBase.BP_EnemyBase_C" (`KismetMathLibrary.Conv_VectorToTransform` (`self.K2_GetActorLocation`)) "Undefined" "MultiplyWithRoot" null null))
    (bind _result (`/Engine/EditorBlueprintResources/StandardMacros.IncrementInt` (`KismetMathLibrary.FTrunc` (`self.BaseDamage`)))
      (:`  `
        (set `self.Slime` _result)
        (goto _label)))))

(event `Take on ground`
  (`SceneComponent.SetVisibility` (`self.StolenCrystal`) true false :!label _label_2)
  (set `self.HoldingCrystal?` true)
  (`KismetSystemLibrary.PrintString` "Crystal held")
  (`|AIMoveTo` self (`self.Start`) null 10.0
    (:`OnSuccess`
      (`self.K2_DestroyActor`))))

(event `self.ReceiveBeginPlay`
  (set `self.Start` (`self.K2_GetActorLocation`))
  (`self.SpawnDefaultController`)
  (`self.Summon Slime!`)
  (bind _returnvalue (`GameplayStatics.GetActorOfClass` "/Game/WinLoseCondition/EnergyCrystals/BP_CrystalCollision.BP_CrystalCollision_C"))
  (`|AIMoveTo` self (`self.K2_GetActorLocation` _returnvalue) null 30.0 :!label _label_3
    (:`OnSuccess`
      (bind _returnvalue_2 (`GameplayStatics.GetActorOfClass` "/Game/WinLoseCondition/EnergyCrystals/BP_CrystalCollision.BP_CrystalCollision_C"))
      (`/Game/WinLoseCondition/EnergyCrystals/BP_CrystalCollision.TakeCrystal` _returnvalue_2)
      (goto _label_2))
    (:`OnFail`
      (`KismetSystemLibrary.Delay` 0.5)
      (goto _label_3))))

(event `self.ReceiveActorBeginOverlap`
  (params (OtherActor :type "Actor Object Reference"))
  (bind _asbp_projectile (cast `/Game/Blueprints/BP_Projectile` OtherActor))
  (`self.K2_DestroyActor` _asbp_projectile)
  (`PrimitiveComponent.SetMaterial` (`self.Mesh`) 0 "/Engine/MapTemplates/Materials/BasicAsset01.BasicAsset01")
  (`KismetSystemLibrary.Delay` 0.2)
  (`PrimitiveComponent.SetMaterial` (`self.Mesh`) 0 (`self.StartMat`))
  (bind _output_get (set `self.HP` (- (`self.HP`) (`self.BaseDamage`))))
  (`KismetSystemLibrary.PrintString` (`KismetStringLibrary.Conv_DoubleToString` _output_get))
  (if (<= _output_get 0.0)
    (if (`self.HoldingCrystal?`)
      (`self.K2_DestroyActor`)
      (`|SpawnActorFromClass` "/Game/WinLoseCondition/EnergyCrystals/BP_EnergyCrystal.BP_EnergyCrystal_C" (`KismetMathLibrary.Conv_VectorToTransform` (`self.K2_GetActorLocation`)) "AdjustIfPossibleButAlwaysSpawn" "MultiplyWithRoot" null null)
      (`KismetSystemLibrary.PrintString` "crystal dropped")
      (else
        (`self.K2_DestroyActor`)))))

(fn `UserConstructionScript`)