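; BP_Spawner is an enemy spawner that runs timed waves of BP_EnemyBase at its own location.
; After a short delay, BeginPlay chains ten Wave calls, each reading enemy count and duration from arrays indexed by WaveIndex.
; Wave sets the player HUD timer, spawns enemies through a delayed loop, then waits out the duration and increments the index.
; An older random-delay endless spawn loop remains unconnected.
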(event `self.ReceiveBeginPlay`
  (bind _output (`|GetArrayItem` (`self.WaveEnemies`) (`self.WaveIndex`)))
  (bind _output_2 (`|GetArrayItem` (`self.WaveLength`) (`self.WaveIndex`)))
  (`KismetSystemLibrary.Delay` 0.2)
  (`self.Wave` _output _output_2)
  (`self.Wave` _output _output_2)
  (`self.Wave` _output _output_2)
  (`self.Wave` _output _output_2)
  (`self.Wave` _output _output_2)
  (`self.Wave` _output _output_2)
  (`self.Wave` _output _output_2)
  (`self.Wave` _output _output_2)
  (`self.Wave` _output _output_2)
  (`self.Wave` _output _output_2))

(fn `UserConstructionScript`)