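; BP_EnemyTurtle is an enemy that steals a crystal and carries it back to its spawn point, where it despawns.
; It moves by AIMoveTo to BP_CrystalCollision, retrying on failure, calls TakeCrystal, then shows the carried crystal.
; Takeonground enters the same carry-and-return path directly.
; Projectile overlaps flash its material and reduce HP; death while carrying spawns a BP_EnergyCrystal drop.
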(event `Take on ground`
  (`SceneComponent.SetVisibility` (`self.StolenCrystal`) true false :!label _label)
  (set `self.HoldingCrystal?` true)
  (`KismetSystemLibrary.PrintString` "Crystal held")
  (`|AIMoveTo` self (`self.Start`) null 10.0
    (:`OnSuccess`
      (`self.K2_DestroyActor`))))

(event `self.ReceiveBeginPlay`
  (set `self.Start` (`self.K2_GetActorLocation`))
  (`self.SpawnDefaultController`)
  (bind _returnvalue (`GameplayStatics.GetActorOfClass` "/Game/WinLoseCondition/EnergyCrystals/BP_CrystalCollision.BP_CrystalCollision_C"))
  (`|AIMoveTo` self (`self.K2_GetActorLocation` _returnvalue) null 30.0 :!label _label_2
    (:`OnSuccess`
      (bind _returnvalue_2 (`GameplayStatics.GetActorOfClass` "/Game/WinLoseCondition/EnergyCrystals/BP_CrystalCollision.BP_CrystalCollision_C"))
      (`/Game/WinLoseCondition/EnergyCrystals/BP_CrystalCollision.TakeCrystal` _returnvalue_2)
      (goto _label))
    (:`OnFail`
      (`KismetSystemLibrary.Delay` 0.5)
      (goto _label_2))))

(event `self.ReceiveActorBeginOverlap`
  (params (OtherActor :type "Actor Object Reference"))
  (bind _asbp_projectile (cast `/Game/Blueprints/BP_Projectile` OtherActor))
  (`self.K2_DestroyActor` _asbp_projectile)
  (`PrimitiveComponent.SetMaterial` (`self.Mesh`) 0 "/Engine/MapTemplates/Materials/BasicAsset01.BasicAsset01")
  (`KismetSystemLibrary.Delay` 0.2)
  (`PrimitiveComponent.SetMaterial` (`self.Mesh`) 0 (`self.Start Material`))
  (bind _output_get (set `self.HP` (- (`self.HP`) (`self.BaseDamage`))))
  (`KismetSystemLibrary.PrintString` (`KismetStringLibrary.Conv_DoubleToString` _output_get))
  (if (<= _output_get 0.0)
    (if (`self.HoldingCrystal?`)
      (`self.K2_DestroyActor`)
      (`|SpawnActorFromClass` "/Game/WinLoseCondition/EnergyCrystals/BP_EnergyCrystal.BP_EnergyCrystal_C" (`KismetMathLibrary.Conv_VectorToTransform` (`self.K2_GetActorLocation`)) "AdjustIfPossibleButAlwaysSpawn" "MultiplyWithRoot" null null)
      (`KismetSystemLibrary.PrintString` "crystal dropped")
      (else
        (`self.K2_DestroyActor`)))))

(fn `UserConstructionScript`)