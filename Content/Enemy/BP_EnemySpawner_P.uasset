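; Enemy spawner actor that releases timed, growing waves of enemies at its own location.
; On BeginPlay it spawns a single BP_EnemyAI, then after fixed delays runs three successively larger loops of BP_EnemyBase spawns.
; Each wave spawns all at once on the same point, and the sequence runs once without repeating or checking whether earlier enemies are dead.
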(event `self.ReceiveBeginPlay`
  (`|SpawnActorFromClass` "/Game/Enemy/BP_EnemyAI.BP_EnemyAI_C" (`KismetMathLibrary.Conv_VectorToTransform` (`self.K2_GetActorLocation`)) "Undefined" "MultiplyWithRoot" null null)
  (`KismetSystemLibrary.Delay` 40.0)
  (for _ (range 11)
    (`|SpawnActorFromClass` "/Game/Enemy/BP_EnemyBase.BP_EnemyBase_C" (`KismetMathLibrary.Conv_VectorToTransform` (`self.K2_GetActorLocation`)) "Undefined" "MultiplyWithRoot" null null))
  (`KismetSystemLibrary.Delay` 30.0)
  (for _ (range 16)
    (`|SpawnActorFromClass` "/Game/Enemy/BP_EnemyBase.BP_EnemyBase_C" (`KismetMathLibrary.Conv_VectorToTransform` (`self.K2_GetActorLocation`)) "Undefined" "MultiplyWithRoot" null null))
  (`KismetSystemLibrary.Delay` 30.0)
  (for _ (range 26)
    (`|SpawnActorFromClass` "/Game/Enemy/BP_EnemyBase.BP_EnemyBase_C" (`KismetMathLibrary.Conv_VectorToTransform` (`self.K2_GetActorLocation`)) "Undefined" "MultiplyWithRoot" null null)))

(fn `UserConstructionScript`)