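; Enemy spawner actor that releases timed waves of BP_EnemyAI_G at its own location.
; BeginPlay spawns a single enemy, then runs a hardcoded chain of six spawn loops of varying size, separated by long Delay pauses.
; Each loop body pairs SpawnActor with a short Delay, and the sequence runs once, with no overlap or Tick logic.
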(event `self.ReceiveBeginPlay`
  (`|SpawnActorFromClass` "/Game/Enemy/BP_EnemyAI_G.BP_EnemyAI_G_C" (`KismetMathLibrary.Conv_VectorToTransform` (`self.K2_GetActorLocation`)) "Undefined" "MultiplyWithRoot" null null)
  (`KismetSystemLibrary.Delay` 35.0)
  (for _ (range 11)
    (`|SpawnActorFromClass` "/Game/Enemy/BP_EnemyAI_G.BP_EnemyAI_G_C" (`KismetMathLibrary.Conv_VectorToTransform` (`self.K2_GetActorLocation`)) "Undefined" "MultiplyWithRoot" null null)
    (`KismetSystemLibrary.Delay` 1.0))
  (`KismetSystemLibrary.Delay` 60.0)
  (for _ (range 11)
    (`|SpawnActorFromClass` "/Game/Enemy/BP_EnemyAI_G.BP_EnemyAI_G_C" (`KismetMathLibrary.Conv_VectorToTransform` (`self.K2_GetActorLocation`)) "Undefined" "MultiplyWithRoot" null null)
    (`KismetSystemLibrary.Delay` 1.0))
  (`KismetSystemLibrary.Delay` 90.0)
  (for _ (range 17)
    (`|SpawnActorFromClass` "/Game/Enemy/BP_EnemyAI_G.BP_EnemyAI_G_C" (`KismetMathLibrary.Conv_VectorToTransform` (`self.K2_GetActorLocation`)) "Undefined" "MultiplyWithRoot" null null)
    (`KismetSystemLibrary.Delay` 1.0))
  (`KismetSystemLibrary.Delay` 30.0)
  (for _ (range 6)
    (`|SpawnActorFromClass` "/Game/Enemy/BP_EnemyAI_G.BP_EnemyAI_G_C" (`KismetMathLibrary.Conv_VectorToTransform` (`self.K2_GetActorLocation`)) "Undefined" "MultiplyWithRoot" null null)
    (`KismetSystemLibrary.Delay` 1.0))
  (`KismetSystemLibrary.Delay` 30.0)
  (for _ (range 13)
    (`|SpawnActorFromClass` "/Game/Enemy/BP_EnemyAI_G.BP_EnemyAI_G_C" (`KismetMathLibrary.Conv_VectorToTransform` (`self.K2_GetActorLocation`)) "Undefined" "MultiplyWithRoot" null null)
    (`KismetSystemLibrary.Delay` 1.0))
  (`KismetSystemLibrary.Delay` 30.0)
  (for _ (range 26)
    (`|SpawnActorFromClass` "/Game/Enemy/BP_EnemyAI_G.BP_EnemyAI_G_C" (`KismetMathLibrary.Conv_VectorToTransform` (`self.K2_GetActorLocation`)) "Undefined" "MultiplyWithRoot" null null)
    (`KismetSystemLibrary.Delay` 1.0)))

(fn `UserConstructionScript`)